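; Game instance Blueprint that owns the game's save data and handles loading and saving it to a named slot.
; On Init it synchronously loads the BPC_SaveGame object into GameData, or creates a new one if none exists.
; Loads and saves support sync or async modes, but only a completed async load fires OnGameLoaded.
; SavePlayerData writes player data into GameData before saving, and GetGameData exposes the cached object.
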(event `self.ReceiveInit`
  (`/Game/Save/BPI_SaveGame.LoadGameData` false))

(event `/Game/Save/BPI_SaveGame.LoadGameData`
  (params (Async :type Boolean))
  (`KismetSystemLibrary.PrintString` "LoadGameData_start")
  (bind _returnvalue (`GameplayStatics.DoesSaveGameExist` (`self.SlotName`)))
  (if _returnvalue
    (if Async
      (bind _savegame (`AsyncActionHandleSaveGame.AsyncLoadGameFromSlot` (`self.SlotName`))
        (:`Completed`
          (bind _asbpc_save_game (cast `/Game/Save/BPC_SaveGame` _savegame))
          (set `self.GameData` _asbpc_save_game)
          (`self.OnGameLoaded`)
          (`KismetSystemLibrary.PrintString` "LoadGameData_end_async")))
      (else
        (bind _returnvalue_2 (`GameplayStatics.LoadGameFromSlot` (`self.SlotName`)))
        (bind _asbpc_save_game_2 (cast `/Game/Save/BPC_SaveGame` _returnvalue_2))
        (set `self.GameData` _asbpc_save_game_2)
        (`KismetSystemLibrary.PrintString` "LoadGameData_end_sync")))
    (else
      (bind _returnvalue_3 (`GameplayStatics.CreateSaveGameObject` "/Game/Save/BPC_SaveGame.BPC_SaveGame_C"))
      (set `self.GameData` _returnvalue_3))))

(event `/Game/Save/BPI_SaveGame.SaveGameData`
  (params (Async :type Boolean))
  (if Async
    (`AsyncActionHandleSaveGame.AsyncSaveGameToSlot` (`self.GameData`) (`self.SlotName`))
    (else
      (`GameplayStatics.SaveGameToSlot` (`self.GameData`) (`self.SlotName`)))))

(event `/Game/Save/BPI_SaveGame.SavePlayerData`
  (params (PlayerData :type "/Game/Save/S_PlayerSave Structure") (Async :type Boolean))
  (set `/Game/Save/BPC_SaveGame.PlayerSave` PlayerData (`self.GameData`))
  (`/Game/Save/BPI_SaveGame.SaveGameData` Async))

(fn `GetGameData`
  (returns (GameData :type "/Game/Save/BPC_SaveGame Object Reference"))
  (return (`self.GameData`)))